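; Menu controller for the additional players (2 to 4) on a character selection screen.
; Select swaps the press prompt for the selection widget and sets that player's flag on MenuRef by PlayerIndex, though player 4's is set false rather than true.
; MoveRight past a deadzone cycles CharacterIndex and image through the main menu's ChangeCharacter, throttled by a DoOnce and short Delay.
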(event `InputAction|Select`
  (params (Key :type "Key Structure" :default "AnyKey"))
  (bind _menuref (`self.MenuRef`))
  (:`Pressed`
    (`Widget.SetVisibility` (`self.MyPress`) "Collapsed")
    (`Widget.SetVisibility` (`self.MySelection`) "Visible")
    (switch `int` (`self.PlayerIndex`)
      (:`1`
        (set `/Game/Blueprints/MenuController.P2` true _menuref))
      (:`2`
        (set `/Game/Blueprints/MenuController.P3` true _menuref))
      (:`3`
        (set `/Game/Blueprints/MenuController.P4` false _menuref)))))

(event `InputAxis|MoveRight`
  (params (AxisValue :type "Float (single-precision)"))
  (bind _myimage (`self.MyImage`))
  (bind _mainmenuref (`/Game/Blueprints/MenuController.MainMenuRef` (`self.MenuRef`)))
  (`/Engine/EditorBlueprintResources/StandardMacros.DoOnce` false :!label _label
    (:`Completed`
      (if (>= AxisValue 0.6)
        (bind _newindexref (`/Game/UI/MainMenuWidget.ChangeCharacter` _mainmenuref (`self.CharacterIndex`) _myimage false))
        (set `self.CharacterIndex` _newindexref)
        (elif (<= AxisValue -0.6)
          (bind _newindexref_2 (`/Game/UI/MainMenuWidget.ChangeCharacter` _mainmenuref (`self.CharacterIndex`) _myimage true))
          (set `self.CharacterIndex` _newindexref_2)))
      (`KismetSystemLibrary.Delay` 0.1)
      (goto _label :!via `Reset`))))

(fn `UserConstructionScript`)