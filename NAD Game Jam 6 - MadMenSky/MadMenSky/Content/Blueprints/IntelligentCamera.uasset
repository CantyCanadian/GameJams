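; Shared race camera for FlyingMadMan players that follows the lowest Y reached and announces the winner.
; BeginPlay registers characters with itself and the HUD, blends two controllers' views here, then starts a looping UpdatePosition timer.
; UpdatePosition also has a kill-line explode check, unreachable once KillScreen updates to 2000 below camera Y.
; Once End is set, Tick shows a win widget naming the position-zero player.
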(event `self.ReceiveTick`
  (params (DeltaSeconds :type "Float (single-precision)"))
  (if (`self.Start`)
    (if (`self.End`)
      (`/Engine/EditorBlueprintResources/StandardMacros.DoOnce` false
        (:`Completed`
          (bind _returnvalue (`|CreateWidget` "/Game/UI/WIN.WIN_C" (`GameplayStatics.GetPlayerController` 0)))
          (for _array_element (`self.CharactersRef`)
            (if (== (`/Game/Character/FlyingMadMan.PlayerPosition` _array_element) 0)
              (`TextBlock.SetText` (`/Game/UI/WIN.WinRef` _returnvalue) (`KismetTextLibrary.Conv_StringToText` (`KismetStringLibrary.Concat_StrStr` "Player " (`KismetStringLibrary.Conv_IntToString` (`/Game/Character/FlyingMadMan.CamRefNumber` _array_element)) " Win")))))
          (`UserWidget.AddToViewport` _returnvalue 0))))))

(event `self.ReceiveBeginPlay`
  (bind (_returnvalue_x _returnvalue_y) (`KismetMathLibrary.BreakVector` (`self.K2_GetActorLocation`)))
  (`KismetSystemLibrary.Delay` 0.1)
  (bind _returnvalue (`|CreateWidget` "/Game/UI/UIPrincipal.UIPrincipal_C" :!label _label))
  (bind _output_get (set `self.WidgetRef` _returnvalue))
  (`UserWidget.AddToViewport` _output_get 0)
  (`KismetSystemLibrary.Delay` 0.02)
  (set `self.XPosition` _returnvalue_y)
  (bind _outactors (`GameplayStatics.GetAllActorsOfClass` "/Game/Character/FlyingMadMan.FlyingMadMan_C"))
  (bind _output_get_2 (set `self.CharactersRef` _outactors))
  (for (_array_element _array_index) _output_get_2
    (set `/Game/Character/FlyingMadMan.CamRef` self _array_element)
    (set `/Game/Character/FlyingMadMan.CamRefNumber` _array_index _array_element)
    (`/Game/UI/UIPrincipal.AssignPlayer` (`self.WidgetRef`) _array_element)
    (set `/Game/Character/FlyingMadMan.HudRef` (`self.WidgetRef`) _array_element)
    (`/Game/Character/FlyingMadMan.NiceLittleFloatingText` _array_element))
  (`PlayerController.SetViewTargetWithBlend` (`GameplayStatics.GetPlayerController` 0) self 0.0 "VTBlend_Linear" 0.0 false)
  (`PlayerController.SetViewTargetWithBlend` (`GameplayStatics.GetPlayerController` 1) self 0.0 "VTBlend_Linear" 0.0 false)
  (`KismetSystemLibrary.K2_SetTimer` self "UpdatePosition" 0.01 true)
  (set `self.Start` true))

(event `StartTheGame`
  (goto _label))

(fn `UpdatePosition`
  (bind (_returnvalue_x _returnvalue_y _returnvalue_z) (`KismetMathLibrary.BreakVector` (`self.K2_GetActorLocation`)))
  (for _array_element (`self.CharactersRef`)
    (bind (_returnvalue_x_2 _returnvalue_y_2) (`KismetMathLibrary.BreakVector` (`self.K2_GetActorLocation` _array_element)))
    (if (< _returnvalue_y_2 (`self.XPosition`))
      (bind _output_get (set `self.XPosition` _returnvalue_y_2))
      (set `self.KillScreen` (- _output_get 2000.0))
      (elif (< _returnvalue_y_2 (`self.KillScreen`))
        (`/Game/Character/FlyingMadMan.Explode` _array_element))))
  (`self.K2_SetActorLocation` (`KismetMathLibrary.MakeVector` _returnvalue_x (`self.XPosition`) _returnvalue_z) false true))

(fn `UserConstructionScript`)