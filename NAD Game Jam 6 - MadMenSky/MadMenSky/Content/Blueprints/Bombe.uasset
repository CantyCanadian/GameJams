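; Bombe is a bomb actor that detonates on contact, spawning a Hiroshima_SideEffects actor at its location and destroying itself.
; On BeginPlay its sphere ignores the instigator during movement, and overlaps with the instigator are likewise skipped.
; Overlap and hit events each have their own DoOnce before detonation.
; A hit also calls Explode on a FlyingMadMan, and only the overlap path passes the instigator to the spawned effect.
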(event `self.ReceiveBeginPlay`
  (`PrimitiveComponent.IgnoreActorWhenMoving` (`self.Sphere`) (`self.GetInstigator`) true))

(event `self.ReceiveActorBeginOverlap`
  (params (OtherActor :type "Actor Object Reference"))
  (bind _returnvalue (`self.GetInstigator`))
  (if (!= OtherActor _returnvalue)
    (`/Engine/EditorBlueprintResources/StandardMacros.DoOnce` false
      (:`Completed`
        (`|SpawnActorFromClass` "/Game/Blueprints/Hiroshima_SideEffects.Hiroshima_SideEffects_C" (`KismetMathLibrary.MakeTransform` (`self.K2_GetActorLocation`) (struct) (1.0 1.0 1.0)) "Undefined" "OverrideRootScale" null _returnvalue)
        (`self.K2_DestroyActor`)))))

(event `self.ReceiveHit`
  (params (MyComp :type "PrimitiveComponent Object Reference") (Other :type "Actor Object Reference") (OtherComp :type "PrimitiveComponent Object Reference") (bSelfMoved :type Boolean) (HitLocation :type "Vector Structure") (HitNormal :type "Vector Structure") (NormalImpulse :type "Vector Structure") (Hit :type "HitResult Structure (by ref)"))
  (bind _asflying_mad_man (cast `/Game/Character/FlyingMadMan` Other)
    (:`then`
      (`/Game/Character/FlyingMadMan.Explode` _asflying_mad_man))
    (:`CastFailed`
      _))
  (`/Engine/EditorBlueprintResources/StandardMacros.DoOnce` false
    (:`Completed`
      (`|SpawnActorFromClass` "/Game/Blueprints/Hiroshima_SideEffects.Hiroshima_SideEffects_C" (`KismetMathLibrary.MakeTransform` (`self.K2_GetActorLocation`) (struct) (1.0 1.0 1.0)) "Undefined" "OverrideRootScale")
      (`self.K2_DestroyActor`))))

(fn `UserConstructionScript`)