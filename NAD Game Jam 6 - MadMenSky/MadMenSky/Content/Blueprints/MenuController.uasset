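; Player one's main menu controller, which creates the menu widget and launches the game from it.
; On BeginPlay it links the other menu controllers to their player panels in the widget.
; Input drives button selection, joining and character cycling, with DoOnce gates throttling the stick.
; Start fires once, hiding the menu, starting the IntelligentCamera and creating players at Spawners by array order for joined slots.
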(event `InputAction|StartInput`
  (params (Key :type "Key Structure" :default "AnyKey"))
  (:`Pressed`
    (`/Engine/EditorBlueprintResources/StandardMacros.DoOnce` false
      (:`Completed`
        (`Widget.SetVisibility` (`self.MainMenuRef`) "Collapsed")
        (bind _outactors (`GameplayStatics.GetAllActorsOfClass` "/Game/Blueprints/IntelligentCamera.IntelligentCamera_C"))
        (`/Game/Blueprints/IntelligentCamera.StartTheGame` (`KismetArrayLibrary.Array_Get` _outactors))
        (bind _outactors_2 (`GameplayStatics.GetAllActorsOfClass` "/Game/Blueprints/Spawner.Spawner_C"))
        (for (_array_element _array_index) _outactors_2
          (switch `int` _array_index
            (:`0`
              (if (`self.P1`)
                (`/Game/Blueprints/Spawner.CreatePlayer` _array_element 0)))
            (:`1`
              (if (`self.P2`)
                (`/Game/Blueprints/Spawner.CreatePlayer` _array_element 0)))
            (:`2`
              (if (`self.P3`)
                (`/Game/Blueprints/Spawner.CreatePlayer` _array_element 0)))
            (:`3`
              (if (`self.P4`)
                (`/Game/Blueprints/Spawner.CreatePlayer` _array_element 0)))))))))

(event `self.ReceiveBeginPlay`
  (bind _mainmenuref (`self.MainMenuRef`))
  (bind _returnvalue (`|CreateWidget` "/Game/UI/MainMenuWidget.MainMenuWidget_C" (`GameplayStatics.GetPlayerController` 0)))
  (set `self.MainMenuRef` _returnvalue)
  (`UserWidget.AddToViewport` _returnvalue 0)
  (for _array_element (`self.OthersRef`)
    (set `/Game/Blueprints/OtherMenuControllers.MenuRef` self _array_element)
    (bind _asother_menu_controllers (cast `/Game/Blueprints/OtherMenuControllers` _array_element))
    (switch `int` (`/Game/Blueprints/OtherMenuControllers.PlayerIndex` _asother_menu_controllers)
      (:`1`
        (set `/Game/Blueprints/OtherMenuControllers.MySelection` (`/Game/UI/MainMenuWidget.P2Panel` _mainmenuref) _asother_menu_controllers)
        (set `/Game/Blueprints/OtherMenuControllers.MyPress` (`/Game/UI/MainMenuWidget.PressA2` _mainmenuref) _asother_menu_controllers)
        (set `/Game/Blueprints/OtherMenuControllers.MyImage` (`/Game/UI/MainMenuWidget.Image_8` _mainmenuref) _asother_menu_controllers))
      (:`2`
        (set `/Game/Blueprints/OtherMenuControllers.MySelection` (`/Game/UI/MainMenuWidget.P3Panel` _mainmenuref) _asother_menu_controllers)
        (set `/Game/Blueprints/OtherMenuControllers.MyPress` (`/Game/UI/MainMenuWidget.PressA3` _mainmenuref) _asother_menu_controllers)
        (set `/Game/Blueprints/OtherMenuControllers.MyImage` (`/Game/UI/MainMenuWidget.P3Select` _mainmenuref) _asother_menu_controllers))
      (:`3`
        (set `/Game/Blueprints/OtherMenuControllers.MySelection` (`/Game/UI/MainMenuWidget.P4Panel` _mainmenuref) _asother_menu_controllers)
        (set `/Game/Blueprints/OtherMenuControllers.MyPress` (`/Game/UI/MainMenuWidget.PressA4` _mainmenuref) _asother_menu_controllers)
        (set `/Game/Blueprints/OtherMenuControllers.MyImage` (`/Game/UI/MainMenuWidget.P4Select` _mainmenuref) _asother_menu_controllers)))))

(event `InputAxis|MoveRight`
  (params (AxisValue :type "Float (single-precision)"))
  (bind _mainmenuref (`self.MainMenuRef`))
  (bind _mainmenuref_2 (`self.MainMenuRef`))
  (bind _image_3 (`/Game/UI/MainMenuWidget.Image_3` _mainmenuref))
  (if (`/Game/UI/MainMenuWidget.SelectedButton` (`self.MainMenuRef`))
    (`/Engine/EditorBlueprintResources/StandardMacros.DoOnce` false :!label _label
      (:`Completed`
        (if (>= AxisValue 0.6)
          (bind _newindexref (`/Game/UI/MainMenuWidget.ChangeCharacter` _mainmenuref (`self.P1CharIndex`) _image_3 false))
          (set `self.P1CharIndex` _newindexref)
          (elif (<= AxisValue -0.6)
            (bind _newindexref_2 (`/Game/UI/MainMenuWidget.ChangeCharacter` _mainmenuref (`self.P1CharIndex`) _image_3 true))
            (set `self.P1CharIndex` _newindexref_2)))
        (`KismetSystemLibrary.Delay` 0.1)
        (goto _label :!via `Reset`)))
    (elif (or (<= AxisValue -0.6) (>= AxisValue 0.6))
      (`/Engine/EditorBlueprintResources/StandardMacros.DoOnce` false :!label _label_2
        (:`Completed`
          (set `/Game/UI/MainMenuWidget.SelectedButton` (not (`/Game/UI/MainMenuWidget.SelectedButton` _mainmenuref_2)) _mainmenuref_2)))
      (else
        (goto _label_2 :!via `Reset`)))))

(event `InputAction|Select`
  (params (Key :type "Key Structure" :default "AnyKey"))
  (bind _mainmenuref (`self.MainMenuRef`))
  (bind _incharacterselect (`/Game/UI/MainMenuWidget.InCharacterSelect` _mainmenuref))
  (:`Pressed`
    (if _incharacterselect
      (`Widget.SetVisibility` (`/Game/UI/MainMenuWidget.P1Panel` _mainmenuref) "Visible")
      (set `self.P1` true)
      (`Widget.SetVisibility` (`/Game/UI/MainMenuWidget.PressA1` _mainmenuref) "Collapsed")
      (else
        (set `/Game/UI/MainMenuWidget.SelectDat` true _mainmenuref))))
  (:`Released`
    (if (not _incharacterselect)
      (set `/Game/UI/MainMenuWidget.SelectDat` false _mainmenuref))))

(fn `UserConstructionScript`)